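; AvoidablePool is an object pool that spawns and recycles side-scrolling obstacles for the player to avoid.
; CreateAvoidable spawns a random class at the right edge up to a cap, with random height and time-scaled random speed, for ThePool.
; UpdateAvoidables moves pooled actors left along X, returning any past the opposite edge to the start with new height and speed.
; Its own event graph is empty.
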(fn `CreateAvoidable`
  (bind _avoidables (`self.avoidables`))
  ;[1 1 1] Only create avoidable if max amount has not been reached
  (if (< (`self.numberOfAvoidable`) (`self.maxNumberofAvoidables`))
    ;[1 1 1] Create avoidable into the scene and adjust its position and speed
    (bind _returnvalue (`|SpawnActorFromClass` (`|GetArrayItem` _avoidables (`KismetMathLibrary.RandomIntegerInRange` 0 (`KismetArrayLibrary.Array_LastIndex` _avoidables))) (`KismetMathLibrary.MakeTransform` (`KismetMathLibrary.MakeVector` (`self.avoidableStartX`) 0.0 (`KismetMathLibrary.RandomFloatInRange` -400.0 1000.0))) "Undefined" "OverrideRootScale" null null))
    (bind _asavoidables (cast `/Game/Blueprints/Avoidables` _returnvalue))
    (bind _speed (`/Game/Blueprints/Collectible.Speed` _asavoidables))
    (set `/Game/Blueprints/Collectible.Speed` (`KismetMathLibrary.RandomFloatInRange` (/ _speed (/ (`KismetSystemLibrary.GetGameTimeInSeconds`) 10.0)) _speed) _asavoidables)
    ;[1 1 1] Add created avoidable to the pool and increment counter
    (`KismetArrayLibrary.Array_Insert` (`self.thePool`) null (`self.numberOfAvoidable`))
    (`/Engine/EditorBlueprintResources/StandardMacros.IncrementInt` (`self.numberOfAvoidable`))))

(fn `UpdateAvoidables`
  (locals (arrayElement :type "/Game/Blueprints/Collectible Object Reference") (arrayIndex :type Integer))
  ;[1 1 1] Update each avoidable in the pool
  (for (_array_element _array_index) (`self.thePool`)
    ;[1 1 1] Check if avoidable has travelled far enough to the left of the screen in order to be valid for reappearing again from the right of the screen
    (set `local.arrayElement` _array_element)
    (set `local.arrayIndex` _array_index)
    (bind _rootcomponent (`Actor.RootComponent` _array_element))
    (if (< (.x (`SceneComponent.K2_GetComponentLocation` _rootcomponent)) (- 0.0 (`self.avoidableStartX`)))
      ;[1 1 1] "Create" avoidable into the scene and adjust its position and speed
      (`SceneComponent.K2_SetWorldLocation` (`Actor.RootComponent` (`local.arrayElement`)) (`KismetMathLibrary.MakeVector` (`self.avoidableStartX`) 0.0 (`KismetMathLibrary.RandomFloatInRange` -400.0 1000.0)) false false)
      (bind _asavoidables (cast `/Game/Blueprints/Avoidables` (`local.arrayElement`)))
      (set `/Game/Blueprints/Collectible.Speed` (`KismetMathLibrary.RandomFloatInRange` 5.0 25.0) _asavoidables)
      (else
        ;[1 1 1] If not too far left, just move the avoidable
        (bind _asavoidables_2 (cast `/Game/Blueprints/Avoidables` _array_element))
        (`SceneComponent.K2_AddWorldOffset` _rootcomponent (`KismetMathLibrary.MakeVector` (- 0.0 (`/Game/Blueprints/Collectible.Speed` _asavoidables_2))) false false)))))

(fn `UserConstructionScript`)