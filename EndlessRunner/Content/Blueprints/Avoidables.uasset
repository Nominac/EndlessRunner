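; Avoidables is an actor Blueprint that triggers an effect when the player character touches it.
; Its Box component's begin-overlap event checks the other actor's display name against "BB_My_Character", then casts it to that class.
; A successful cast calls ApplyEffect with the character, and that effect's logic is not defined in these graphs.
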(event `self.Box.OnComponentBeginOverlap`
  (params (OverlappedComponent :type "PrimitiveComponent Object Reference") (OtherActor :type "Actor Object Reference") (OtherComp :type "PrimitiveComponent Object Reference") (OtherBodyIndex :type Integer) (bFromSweep :type Boolean) (SweepResult :type "HitResult Structure (by ref)"))
  ;[1 1 1] Check whether collectible begins to overlap player character
  (if (`KismetStringLibrary.EqualEqual_StrStr` (`KismetSystemLibrary.GetDisplayName` OtherActor) "BB_My_Character")
    (bind _asbb_my_character (cast `/Game/Blueprints/BB_My_Character` OtherActor))
    (`self.ApplyEffect` _asbb_my_character)))

(fn `UserConstructionScript`
  (`parent.UserConstructionScript`))