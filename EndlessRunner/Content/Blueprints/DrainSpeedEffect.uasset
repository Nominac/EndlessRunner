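; DrainSpeedEffect is an avoidable whose effect slows the player by draining horizontal speed.
; ApplyEffect subtracts SpeedDrain from the player's XSpeed only when the result stays above zero.
; A successful drain also records the effect start time on the player and sets the avoidable's own Speed to move it out of view.
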(event `self.ApplyEffect`
  (params (PlayerCharacter :type "/Game/Blueprints/BB_My_Character Object Reference"))
  (bind _returnvalue (- (`/Game/Blueprints/BB_My_Character.XSpeed` PlayerCharacter) (`self.speedDrain`)))
  ;[1 1 1] Apply drain effect; decrease player's horizontal speed
  (set `self.thePlayer` PlayerCharacter)
  (if (> _returnvalue 0.0)
    (set `/Game/Blueprints/BB_My_Character.XSpeed` _returnvalue (`self.thePlayer`))
    ;[1 1 1] Set start time for the drain speed effect
    (set `/Game/Blueprints/BB_My_Character.effectStartTime` (`KismetSystemLibrary.GetGameTimeInSeconds`) (`self.thePlayer`))
    (set `self.Speed` 500.0) ; Move the avoidable out of the picture
  ))

(fn `UserConstructionScript`
  (`parent.UserConstructionScript`))