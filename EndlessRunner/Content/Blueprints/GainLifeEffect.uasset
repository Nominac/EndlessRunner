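; GainLifeEffect is an effect Blueprint that restores the player character's life force when ApplyEffect is called.
; It acts only when life force is below the 1.0 maximum, and clamps the result to that cap.
; The boost is the Effect value scaled by elapsed game time, so the heal grows larger the longer the game runs.
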(event `self.ApplyEffect`
  (params (PlayerCharacter :type "/Game/Blueprints/BB_My_Character Object Reference"))
  (bind _lifeforce (`/Game/Blueprints/BB_My_Character.lifeForce` PlayerCharacter))
  (bind _returnvalue (+ _lifeforce (* (/ (`KismetSystemLibrary.GetGameTimeInSeconds`) 5.0) (`self.Effect`))))
  ;[1 1 1] Check if player's life force is not on maximum before boost
  (if (< _lifeforce 1.0)
    ;[1 1 1] Check if sum of boost and life force is on maximum
    (if (<= _returnvalue 1.0)
      (set `/Game/Blueprints/BB_My_Character.lifeForce` _returnvalue PlayerCharacter)
      (else
        (set `/Game/Blueprints/BB_My_Character.lifeForce` 1.0 PlayerCharacter)))))

(fn `UserConstructionScript`
  (`parent.UserConstructionScript`))